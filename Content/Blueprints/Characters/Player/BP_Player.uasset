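; BP_Player is the player character Blueprint, handling input setup and a mouse-driven interact trace.
; BeginPlay adds the IMC_Inputs Enhanced Input mapping context through the BP_PlayerController.
; The interact action runs a debug-drawn Visibility trace from the deprojected cursor position to its scaled direction, without adding the start position.
; A hit actor gets an interface check, but nothing follows it yet.
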(event `self.ReceiveBeginPlay`
  ; Input mapping
  (bind _asbp_player_controller (cast `/Game/Blueprints/BP_PlayerController` (`self.GetController`)))
  (bind _returnvalue (pcsubsystem `EnhancedInputLocalPlayerSubsystem` _asbp_player_controller))
  (`/Engine/EditorBlueprintResources/StandardMacros.IsValid` _returnvalue
    (:`Is Valid`
      (`EnhancedInputSubsystemInterface.AddMappingContext` _returnvalue "/Game/Inputs/IMC_Inputs.IMC_Inputs" 0 (struct)))))

(event `EnhancedInput|/Game/Inputs/AI_Interact`
  (params (ActionValue :type Boolean) (ElapsedSeconds :type "Float (double-precision)") (TriggeredSeconds :type "Float (double-precision)") (InputAction :type "InputAction Object Reference" :default "/Game/Inputs/AI_Interact.AI_Interact"))
  (bind (_worldlocation _worlddirection) (`PlayerController.DeprojectMousePositionToWorld` (`GameplayStatics.GetPlayerController` 0)))
  (:`Triggered`
    (bind (_outhit _returnvalue) (`KismetSystemLibrary.LineTraceSingle` :`Start` _worldlocation :`End` (* _worlddirection 10000.0) :`TraceChannel` "TraceTypeQuery1" :`DrawDebugType` "ForDuration"))
    (if _returnvalue
      (if (`KismetSystemLibrary.DoesImplementInterface` (`.HitActor` (`GameplayStatics.BreakHitResult` _outhit)))
        _))))

(fn `UserConstructionScript`)